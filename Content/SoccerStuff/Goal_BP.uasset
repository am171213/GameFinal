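; Soccer goal Blueprint that detects when the ball enters it and awards a point.
; A box overlap filters for SoccerBallBP, then updates the score and activates a particle effect.
; UpdateScore increments player one or player two's score on the ScoreHUD based on BelongsToPlayer.
; The construction script applies the Color material to the three goal meshes.
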(event OnComponentBeginOverlap(Box)
  (params (OverlappedComponent :type Primitive%20Component%20Object%20Reference) (OtherActor :type Actor%20Object%20Reference) (OtherComp :type Primitive%20Component%20Object%20Reference) (OtherBodyIndex :type Integer) (bFromSweep :type Boolean) (SweepResult :type Hit%20Result%20Structure%20%28by%20ref%29))
  ;[1 1 1] Soccer Ball In Goal
  (Utilities|Casting|CastToSoccerBallBP OtherActor)
  (CallFunction|UpdateScore)
  (Components|Activation|Activate (Variables|Default|GetParticleSystem) true))

(fn ConstructionScript
  (bind _color (Variables|Default|GetColor))
  (Rendering|Material|SetMaterial (Variables|Default|GetStaticMesh) 0 _color)
  (Rendering|Material|SetMaterial (Variables|Default|GetStaticMesh1) 0 _color)
  (Rendering|Material|SetMaterial (Variables|Default|GetStaticMesh2) 0 _color))

(fn UpdateScore
  ;[1 1 1] PlayerScored
  (if (== (Variables|Default|GetBelongsToPlayer) 1)
    (Math|Integer|IncrementInt (Variables|/Game/SoccerStuff/SoccerHUD.SoccerHUD_C|GetP1Score (Variables|Default|GetScore%20HUD)))
    (else
      (Math|Integer|IncrementInt (Variables|/Game/SoccerStuff/SoccerHUD.SoccerHUD_C|GetP2Score (Variables|Default|GetScore%20HUD))))))